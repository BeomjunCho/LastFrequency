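; Player inventory component that holds a fixed-size array of item structs and drives the W_InventoryGrid widget.
; BeginPlay creates the grid; IA_Inventory only opens it, switching to UI-only input with the cursor shown.
; F sphere-traces near the player's feet for a BP_Item, then walks the slots to stack it within the per-item limit or fill an empty one.
; A successful pickup refreshes the grid and destroys the world actor.
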(event Input|EnhancedActionEvents|EnhancedInputActionIA_Inventory
  (params (ActionValue :type Boolean) (ElapsedSeconds :type Float%20%28double-precision%29) (TriggeredSeconds :type Float%20%28double-precision%29) (InputAction :type Input%20Action%20Object%20Reference :default "/Game/FirstPerson/Input/Actions/IA_Inventory.IA_Inventory"))
  (bind _returnvalue (Game|GetPlayerController 0))
  (bind _inventorywidgetreference (Variables|Default|GetInventoryWidgetReference))
  (if (not (Widget|IsVisible (Variables|Default|GetInventoryWidgetReference)))
    (UserInterface|Viewport|AddtoViewport (Variables|Default|GetInventoryWidgetReference) 0)
    (Variables|/Script/Engine.PlayerController|SetbShowMouseCursor _returnvalue true)
    (Input|SetInputModeUIOnly _returnvalue _inventorywidgetreference "DoNotLock" false)
    (Variables|/Script/UMG.UserWidget|SetbIsFocusable _inventorywidgetreference true)))

(event EventBeginPlay
  (bind _returnvalue (UserInterface|CreateWidget "/Game/LastFrequency/Systems/InventorySystem/Widgets/W_InventoryGrid.W_InventoryGrid_C"))
  (Variables|Default|SetInventoryWidgetReference _returnvalue)
  (Utilities|Array|Resize (Variables|Default|GetInvItems) (Variables|Default|GetInvSize))
  (Default|RefreshInventory (Variables|Default|GetInventoryWidgetReference) self))

(event Input|KeyboardEvents|C
  (params (Key :type Key%20Structure :default "None")))

(event Input|KeyboardEvents|F
  (params (Key :type Key%20Structure :default "None"))
  (bind _returnvalue (Game|GetPlayerCharacter 0))
  (bind _returnvalue_2 (Transformation|GetActorLocation _returnvalue))
  (bind _returnvalue_3 (- _returnvalue_2 "0.000000,0.000000,65.000000"))
  (:Pressed
    (bind _outhit (Collision|SphereTraceByChannel _returnvalue_3 _returnvalue_3 1.2e+02 "TraceTypeQuery1" false 0 "None"))
    (bind _asbp_item (Utilities|Casting|CastToBP_Item (.HitActor (Collision|BreakHitResult _outhit))))
    (for (_array_element _array_index) (Variables|Default|GetInvItems)
      (Utilities|IsValid _asbp_item
        (:Is%20Valid
          (if (Math|Boolean|ANDBoolean (Utilities|Enum|Equal(Enum) (.ItemName (Utilities|Struct|BreakS_Item _array_element)) (.ItemName (Utilities|Struct|BreakS_Item (Variables|/Game/LastFrequency/Systems/InventorySystem/Blueprints/BP_Item.BP_Item_C|GetStItem _asbp_item)))) (.ItemStackable? (Utilities|Struct|BreakS_Item (Variables|/Game/LastFrequency/Systems/InventorySystem/Blueprints/BP_Item.BP_Item_C|GetStItem _asbp_item))) (<= (+ (.ItemAmount (Utilities|Struct|BreakS_Item _array_element)) (.ItemAmount (Utilities|Struct|BreakS_Item (Variables|/Game/LastFrequency/Systems/InventorySystem/Blueprints/BP_Item.BP_Item_C|GetStItem _asbp_item)))) (Variables|Default|GetMaxAmountPerItem)))
            (Utilities|Array|SetArrayElem (Variables|Default|GetInvItems) _array_index (Utilities|Struct|MakeS_Item (.iteminventory? (Variables|/Game/LastFrequency/Systems/InventorySystem/Blueprints/BP_Item.BP_Item_C|GetStItem _asbp_item)) (.itemname (Variables|/Game/LastFrequency/Systems/InventorySystem/Blueprints/BP_Item.BP_Item_C|GetStItem _asbp_item)) (.itemdescription (Variables|/Game/LastFrequency/Systems/InventorySystem/Blueprints/BP_Item.BP_Item_C|GetStItem _asbp_item)) (.itemstackable? (Variables|/Game/LastFrequency/Systems/InventorySystem/Blueprints/BP_Item.BP_Item_C|GetStItem _asbp_item)) (+ (.ItemAmount (Utilities|Struct|BreakS_Item _array_element)) (.ItemAmount (Utilities|Struct|BreakS_Item (Variables|/Game/LastFrequency/Systems/InventorySystem/Blueprints/BP_Item.BP_Item_C|GetStItem _asbp_item)))) (.itemmesh (Variables|/Game/LastFrequency/Systems/InventorySystem/Blueprints/BP_Item.BP_Item_C|GetStItem _asbp_item)) (.itemimage (Variables|/Game/LastFrequency/Systems/InventorySystem/Blueprints/BP_Item.BP_Item_C|GetStItem _asbp_item))))
            (Variables|/Game/LastFrequency/Systems/InventorySystem/Blueprints/BP_Item.BP_Item_C|SetStItem _asbp_item (Utilities|Struct|MakeS_Item (.iteminventory? (Variables|/Game/LastFrequency/Systems/InventorySystem/Blueprints/BP_Item.BP_Item_C|GetStItem _asbp_item)) (.itemname (Variables|/Game/LastFrequency/Systems/InventorySystem/Blueprints/BP_Item.BP_Item_C|GetStItem _asbp_item)) (.itemdescription (Variables|/Game/LastFrequency/Systems/InventorySystem/Blueprints/BP_Item.BP_Item_C|GetStItem _asbp_item)) (.itemstackable? (Variables|/Game/LastFrequency/Systems/InventorySystem/Blueprints/BP_Item.BP_Item_C|GetStItem _asbp_item)) (+ (.ItemAmount (Utilities|Struct|BreakS_Item _array_element)) (.ItemAmount (Utilities|Struct|BreakS_Item (Variables|/Game/LastFrequency/Systems/InventorySystem/Blueprints/BP_Item.BP_Item_C|GetStItem _asbp_item)))) (.itemmesh (Variables|/Game/LastFrequency/Systems/InventorySystem/Blueprints/BP_Item.BP_Item_C|GetStItem _asbp_item)) (.itemimage (Variables|/Game/LastFrequency/Systems/InventorySystem/Blueprints/BP_Item.BP_Item_C|GetStItem _asbp_item))))
            (Default|RefreshInventory (Variables|Default|GetInventoryWidgetReference) self :!label _label)
            (Actor|DestroyActor _asbp_item)
            (elif (== (.ItemAmount (Utilities|Struct|BreakS_Item _array_element)) 0)
              (Utilities|Array|SetArrayElem (Variables|Default|GetInvItems) _array_index (Variables|/Game/LastFrequency/Systems/InventorySystem/Blueprints/BP_Item.BP_Item_C|GetStItem _asbp_item))
              (goto _label))))))))