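; BP_Item is an item actor in the inventory system that represents an item in the world as a physics-simulated static mesh.
; Its construction script applies the mesh from the StItem struct and turns on physics simulation.
; The event graph is empty, while debug visibility toggling, item scaling and the inner and outer sphere radius values are left disconnected or unused.
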(event EventBeginPlay)

(event Collision|EventActorBeginOverlap
  (params (OtherActor :type Actor%20Object%20Reference)))

(event EventTick
  (params (DeltaSeconds :type Float%20%28single-precision%29)))

(fn ConstructionScript
  (bind _staticmesh (Variables|Default|GetStaticMesh))
  (Utilities|FlowControl|Sequence
    (:then_1
      (Components|StaticMesh|SetStaticMesh _staticmesh (.ItemMesh (Utilities|Struct|BreakS_Item (Variables|Inventory|GetStItem))))
      (Physics|SetSimulatePhysics _staticmesh true))))