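; BP_AudioPuzzle2 is a proximity-activated trigger that opens the second audio puzzle for the player.
; A box overlap with the first-person character shows or hides the activation text and toggles whether interaction is allowed.
; While allowed, pressing F creates the WBP_AudioPuzzle2 widget with a countdown value, adds it to the viewport, shows the cursor and switches input to UI-only.
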(event OnComponentBeginOverlap(Box)
  (params (OverlappedComponent :type Primitive%20Component%20Object%20Reference) (OtherActor :type Actor%20Object%20Reference) (OtherComp :type Primitive%20Component%20Object%20Reference) (OtherBodyIndex :type Integer) (bFromSweep :type Boolean) (SweepResult :type Hit%20Result%20Structure%20%28by%20ref%29))
  (Utilities|Casting|CastToBP_FirstPersonCharacter OtherActor)
  (Rendering|SetVisibility (Variables|Default|GetText_Activate) true false)
  (Variables|Default|SetCanAcitve true))

(event OnComponentEndOverlap(Box)
  (params (OverlappedComponent :type Primitive%20Component%20Object%20Reference) (OtherActor :type Actor%20Object%20Reference) (OtherComp :type Primitive%20Component%20Object%20Reference) (OtherBodyIndex :type Integer))
  (Utilities|Casting|CastToBP_FirstPersonCharacter OtherActor)
  (Rendering|SetVisibility (Variables|Default|GetText_Activate) false false)
  (Variables|Default|SetCanAcitve false))

(event EventBeginPlay
  (Input|EnableInput (Game|GetPlayerController 0)))

(event Collision|EventActorBeginOverlap
  (params (OtherActor :type Actor%20Object%20Reference)))

(event EventTick
  (params (DeltaSeconds :type Float%20%28single-precision%29)))

(event Input|KeyboardEvents|F
  (params (Key :type Key%20Structure :default "None"))
  (bind _returnvalue (Game|GetPlayerController 0))
  ;[1 1 1] Create widget and play wwise event
  (:Pressed
    (if (Variables|Default|GetCanAcitve)
      (bind _returnvalue_2 (UserInterface|CreateWidget "/Game/LastFrequency/Systems/AudioPuzzle/Puzzle2/Widget/WBP_AudioPuzzle2.WBP_AudioPuzzle2_C" 0 (Variables|Default|GetCountDown)))
      (bind _output_get (Variables|Default|SetWBP%20Audio%20Puzzle2 _returnvalue_2))
      (UserInterface|Viewport|AddtoViewport _output_get 0)
      (Variables|/Script/Engine.PlayerController|SetbShowMouseCursor _returnvalue true)
      (Input|SetInputModeUIOnly _returnvalue (Variables|Default|GetWBP%20Audio%20Puzzle2) "DoNotLock" false))))

(fn ConstructionScript
  (Rendering|SetVisibility (Variables|Default|GetText_Activate) false false))